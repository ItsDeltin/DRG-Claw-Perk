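; BP_Claw is the hand-held claw actor for a Deep Rock Galactic claw perk, attached to the dwarf's first-person left hand and used to fire a hook.
; It assembles handle, shaft, pommel and head pieces from pickaxe parts using the player's DRG context, with an editor-only construction-script preview from test parts.
; The server spawns and owns the BP_Hook lifecycle, destroying it with the claw.
; Fire forwards to the hook's FireServer.
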(event `self.ReceiveBeginPlay`
  (bind _hook_args (`self.Hook Args`))
  ;[1 0.03646 0.03646] Begin Play
  (`/Game/ClawPerk/BP_ClawFunctionLibrary.Make Pieces from DRG Context` (`.DRGContext_23_E46872554C41985D51C363B53E8BAA09` (break `/Game/ClawPerk/F_MakeHookArgs` _hook_args)) (`self.Handle`) (`self.Get Model Pieces`) (`/Game/ClawPerk/BP_ClawFunctionLibrary.Get Editor Pickaxe Part Testing Array`))
  (`self.Attach To Hand`)
  ;;[1 0.7094 0.06849] Spawn Hook (Server)
  (`/Engine/EditorBlueprintResources/ActorMacros.Switch Has Authority`
    (:`Authority`
      (bind _returnvalue (`|SpawnActorFromClass` "/Game/ClawPerk/BP_Hook.BP_Hook_C" (`KismetMathLibrary.MakeTransform` (0.0 0.0 0.0)) "Undefined" "OverrideRootScale" self _hook_args (0.0 0.0 0.0) self null))
      (set `self.Hook` _returnvalue))))

(event `self.ReceiveDestroyed`
  (`/Engine/EditorBlueprintResources/ActorMacros.Switch Has Authority`
    (:`Authority`
      (`self.K2_DestroyActor` (`self.Hook`)))))

(event `self.ReceiveTick`
  (params (DeltaSeconds :type "Float (single-precision)")))

(fn `Attach To Hand`
  (bind (_drgcontext_drgcontextavailable _drgcontext_drgperkasset _drgcontext_drgplayercharacter) (break `/Game/ClawPerk/F_DrgContext` (break `/Game/ClawPerk/F_MakeHookArgs` (`self.Hook Args`))))
  (bind _fpmesh (`PlayerCharacter.FPMesh` _drgcontext_drgplayercharacter))
  (bind _returnvalue_location (`KismetMathLibrary.BreakTransform` (`SceneComponent.GetSocketTransform` _fpmesh "Dwarf_HandL_Attach" "RTS_ParentBoneSpace")))
  (if _drgcontext_drgcontextavailable
    (`self.K2_AttachToComponent` _fpmesh "Dwarf_HandL_Attach" "KeepRelative" "KeepRelative" "KeepRelative")
    (`self.K2_SetActorRelativeTransform` (`KismetMathLibrary.MakeTransform` (* _returnvalue_location (-2.0 -2.0 1.0))))))

(fn `Fire`
  (`/Game/ClawPerk/BP_Hook.Fire Server` (`self.Hook`)))

(fn `Get Model Pieces`
  (returns (Pieces :type "Array of /Game/ClawPerk/F_ClawPiece Structure"))
  (return (`|MakeArray` (make `/Game/ClawPerk/F_ClawPiece` "Handle" "None" (`self.RT Grabber Handle`)) (make `/Game/ClawPerk/F_ClawPiece` "Shaft" "None" (`self.RT Grabber Shaft`)) (make `/Game/ClawPerk/F_ClawPiece` "Pommel" "None" (`self.RT Grabber Pommel`)) (make `/Game/ClawPerk/F_ClawPiece` "Head" "None" (`self.RT Grabber Head`)))))

(fn `UserConstructionScript`
  (if (not (`KismetSystemLibrary.IsPackagedForDistribution`))
    (`/Game/ClawPerk/BP_ClawFunctionLibrary.Make Pieces` (`/Game/ClawPerk/BP_ClawFunctionLibrary.Get Editor Pickaxe Part Testing Array`) null (`self.Handle`) (`self.Get Model Pieces`))))