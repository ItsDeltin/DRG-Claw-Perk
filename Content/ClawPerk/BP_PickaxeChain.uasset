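; Claw perk chain actor that draws a chain of alternating pickaxe handle and head meshes between itself and its End component.
; Each Tick spreads the spline points evenly between both ends, adding per-point recoil offsets.
; It then walks the spline back from its far end, aligning collision-free static mesh links along it.
; Existing links are reused, with components added or destroyed as length changes, up to a maximum count.
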(event `self.ReceiveBeginPlay`
  (`self.Init Spline` 6))

(event `self.ReceiveTick`
  (params (DeltaSeconds :type "Float (single-precision)"))
  (bind _chain_pieces (`self.Chain Pieces`))
  (bind _apply_chain_distance (`self.Apply Chain Distance`))
  (bind _scale (`self.Scale`))
  (bind _current_chain_length (`self.Current Chain Length`))
  (bind _spline (`self.Spline`))
  (bind _apply_chain_index (`self.Apply Chain Index`))
  (bind _returnvalue (- _current_chain_length 1))
  (bind (_out_index _origin_offset _length _skip _debug_name _static_mesh) (`self.Get Chain Link From Index` _apply_chain_index))
  (bind _returnvalue_2 (`SplineComponent.GetLocationAtDistanceAlongSpline` _spline _apply_chain_distance "Local"))
  (bind _returnvalue_3 (`KismetMathLibrary.FindLookAtRotation` _returnvalue_2 (`SplineComponent.GetLocationAtDistanceAlongSpline` _spline (- _apply_chain_distance _length) "Local")))
  (bind _returnvalue_4 (`KismetMathLibrary.MakeTransform` (+ (* (`KismetMathLibrary.GetForwardVector` _returnvalue_3) _origin_offset) _returnvalue_2) (`KismetMathLibrary.ComposeRotators` (struct :`Pitch` -90.0) _returnvalue_3) (`KismetMathLibrary.MakeVector` _scale _scale _scale)))
  (`self.Update Spline Points` DeltaSeconds)
  (set `self.Apply Chain Index` 0) ; Initialize ApplyChainIndex
  (set `self.Apply Chain Distance` (`SplineComponent.GetSplineLength` _spline)) ; Initialize ApplyChainDistance
  (while (and (> (`self.Apply Chain Distance`) 0.0) (< (`self.Apply Chain Index`) (`self.Maximum Chain Count`)))
    (if (< _apply_chain_index (`self.Current Chain Length`))
      (`SceneComponent.K2_SetRelativeTransform` (`|GetArrayItem` (`self.Chain Pieces`) (`self.Apply Chain Index`)) _returnvalue_4 false false)
      (else
        (bind _returnvalue_5 (`|AddComponentByClass` "/Script/Engine.StaticMeshComponent" false _returnvalue_4))
        (`StaticMeshComponent.SetStaticMesh` _returnvalue_5 _static_mesh)
        (`PrimitiveComponent.SetMaterial` _returnvalue_5 0 (`self.Pickaxe Material`))
        (`PrimitiveComponent.SetCollisionEnabled` _returnvalue_5 "NoCollision")
        (`KismetArrayLibrary.Array_Add` (`self.Chain Pieces`) _returnvalue_5)
        (`/Engine/EditorBlueprintResources/StandardMacros.IncrementInt` (`self.Current Chain Length`)
          (:`  `
            _))))
    (bind _output_get (set `self.Apply Chain Distance` (- (stale _output_get) _skip)))
    (`/Engine/EditorBlueprintResources/StandardMacros.IncrementInt` (`self.Apply Chain Index`)))
  (while (< (`self.Apply Chain Index`) _current_chain_length)
    (`ActorComponent.K2_DestroyComponent` (`|GetArrayItem` _chain_pieces _returnvalue))
    (`KismetArrayLibrary.Array_Remove` _chain_pieces _returnvalue)
    (`/Engine/EditorBlueprintResources/StandardMacros.DecrementInt` _current_chain_length)))

(fn `Get Chain Link From Index`
  (params (Index :type Integer))
  (returns (`Out Index` :type Integer) (`Origin Offset` :type "Float (double-precision)") (Length :type "Float (double-precision)") (Skip :type "Float (double-precision)") (`Debug Name` :type String) (`Static Mesh` :type "StaticMesh Object Reference"))
  (locals (`Chosen Offset` :type "Float (double-precision)") (`Chosen Length` :type "Float (double-precision)") (`Chosen Skip` :type "Float (double-precision)") (`Chosen Name` :type String) (`Chosen Mesh` :type "StaticMesh Object Reference"))
  (bind _scale (`self.Scale`))
  (switch `int` (mod Index 2)
    (:`0`
      (set `local.Chosen Offset` (`self.Handle Origin Offset`))
      (set `local.Chosen Length` (`self.Handle Length`))
      (set `local.Chosen Skip` (`self.Handle Skip`))
      (set `local.Chosen Name` "Handle")
      (set `local.Chosen Mesh` (`self.Handle Mesh`)))
    (:`1`
      (set `local.Chosen Offset` (`self.Head Origin Offset`))
      (set `local.Chosen Length` (`self.Head Length`))
      (set `local.Chosen Skip` (`self.Head Skip`))
      (set `local.Chosen Name` "Head")
      (set `local.Chosen Mesh` (`self.Head Mesh`))))
  (return (/ Index 2) (* (`local.Chosen Offset`) _scale) (* (`local.Chosen Length`) _scale) (* (`local.Chosen Skip`) _scale) "Handle" (`local.Chosen Mesh`)))

(fn `Init Spline`
  (params (`Number of points` :type Integer))
  (locals (points :type "Array of Vector Structure"))
  (for _index (range (+ `Number of points` 1))
    (`KismetArrayLibrary.Array_Add` (`local.points`) (`KismetMathLibrary.MakeVector` (`KismetMathLibrary.Conv_IntToDouble` _index)))
    (`KismetArrayLibrary.Array_Add` (`self.Hook Recoil Offsets`)))
  (`SplineComponent.SetSplinePoints` (`self.Spline`) (`local.points`) "Local" true))

(fn `Update Spline Points`
  (params (`Delta Seconds` :type "Float (double-precision)"))
  (bind _returnvalue (`self.K2_GetActorLocation`))
  (bind _spline (`self.Spline`))
  (bind _returnvalue_2 (- (`SplineComponent.GetNumberOfSplinePoints` (`self.Spline`)) 1))
  (for _index (range (+ _returnvalue_2 1))
    (`SplineComponent.SetLocationAtSplinePoint` _spline _index (+ (* (- (`SceneComponent.K2_GetComponentLocation` (`self.End`)) _returnvalue) (/ (`KismetMathLibrary.Conv_IntToDouble` _index) (`KismetMathLibrary.Conv_IntToDouble` _returnvalue_2))) _returnvalue (`|GetArrayItem` (`self.Hook Recoil Offsets`) _index)) "World" false))
  (`SplineComponent.UpdateSpline` _spline))

(fn `UserConstructionScript`)