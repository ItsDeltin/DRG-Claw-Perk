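; Deep Rock Galactic perk claw, built from the player's pickaxe parts, that shoots from the hand to a target actor and hauls it back.
; A state machine runs extend, recoil and retract, bending a spline with randomized timeline offsets.
; Tick lays alternating handle and head meshes along the spline as chain.
; The server sweeps the grabbed actor along; release spends a perk charge and picks up, uses or frees it by type.
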(event `self.ReceiveBeginPlay`
  (set `self.Current Location` (`self.Source Location`))
  (`self.Init Spline` 10)
  (`SkeletalMeshComponent.PlayAnimation` (`self.Grabber`) "/Game/ClawPerk/ClawAsset/Grabber_Anim_Ready.Grabber_Anim_Ready" false))

(event `self.ReceiveTick`
  (params (DeltaSeconds :type "Float (single-precision)"))
  (bind _spline (`self.Spline`))
  (bind _apply_chain_distance (`self.Apply Chain Distance`))
  (bind _spline_2 (`self.Spline`))
  (bind _apply_chain_index (`self.Apply Chain Index`))
  (bind _returnvalue (`SplineComponent.GetLocationAtDistanceAlongSpline` _spline_2 _apply_chain_distance "Local"))
  (bind (_instance_static_mesh_component _out_index _origin_offset _length _skip _debug_name _static_mesh) (`self.Get Chain Link From Index` _apply_chain_index))
  (bind _returnvalue_2 (`SplineComponent.GetNumberOfSplinePoints` _spline))
  (bind _returnvalue_3 (`KismetMathLibrary.FindLookAtRotation` _returnvalue (`SplineComponent.GetLocationAtDistanceAlongSpline` _spline_2 (- _apply_chain_distance _length) "Local")))
  (bind _returnvalue_4 (`KismetMathLibrary.MakeTransform` (+ (* (`KismetMathLibrary.GetForwardVector` _returnvalue_3) _origin_offset) _returnvalue) (`KismetMathLibrary.ComposeRotators` (struct :`Pitch` -90.0) _returnvalue_3)))
  (`|ExecutionSequence`
    (:`then_0`
      (`self.Update Spline Points` DeltaSeconds))
    (:`then_1`
      (switch `/Game/ClawPerk/E_ClawState` (`self.State`)
        (:`NewEnumerator0`
          (if (`self.Is destination reached`)
            (set `self.State` "NewEnumerator1")
            (`self.Grab Target`)
            (`SkeletalMeshComponent.PlayAnimation` (`self.Grabber`) "/Game/ClawPerk/ClawAsset/Grabber_Anim_Grab.Grabber_Anim_Grab" false)
            (set `self.Hook Recoil` (`|MakeMap`))
            (for _index (range (- _returnvalue_2 4) (+ (- _returnvalue_2 3) 1))
              (`BlueprintMapLibrary.Map_Add` (`self.Hook Recoil`) _index (make `/Game/ClawPerk/F_HookRecoil` _index (+ (* (`KismetMathLibrary.GetForwardVector` (`SplineComponent.GetRotationAtSplinePoint` _spline _index "Local")) (* (`KismetMathLibrary.Conv_IntToDouble` (- _returnvalue_2 _index)) 20.0)) (`KismetMathLibrary.MakeVector` (`KismetMathLibrary.RandomFloatInRange` -50.0 50.0) (`KismetMathLibrary.RandomFloatInRange` -50.0 50.0) (`KismetMathLibrary.RandomFloatInRange` -50.0 50.0))))))
            (bind _values (`BlueprintMapLibrary.Map_Values` (`self.Hook Recoil`)))
            (bind (_direction _recoil_lerp) (`Timeline|TimeLine` :!via `PlayFromStart`)
              (:`Update`
                (for _array_element _values
                  (bind ((`SplicePointIndex_2_9C4F98CD4CE9E8B2F4BF8990C0F5DE8C` _splicepointindex) (`DestinationPoint_7_40F4EC264B83133A3561AAA762478353` _destinationpoint)) (break `/Game/ClawPerk/F_HookRecoil` _array_element))
                  (`KismetArrayLibrary.Array_Set` (`self.Hook Recoil Offsets`) _splicepointindex (`KismetMathLibrary.VLerp` (0.0 0.0 0.0) _destinationpoint _recoil_lerp) true)))
              (:`Finished`
                (set `self.State` "NewEnumerator2")))))
        (:`NewEnumerator2`
          (`self.Update Grabbed Target`)
          (if (`self.Is destination reached`)
            (set `self.State` "NewEnumerator3")
            (`self.Release Target`)
            (`self.K2_DestroyActor`)))))
    (:`then_2`
      (if (not (`self.IsActorBeingDestroyed`))
        (`|ExecutionSequence`
          (:`then_0`
            (set `self.Apply Chain Index` 0) ; Initialize ApplyChainIndex
            (set `self.Apply Chain Distance` (`SplineComponent.GetSplineLength` _spline_2)) ; Initialize ApplyChainDistance
            (while (and (> (`self.Apply Chain Distance`) 0.0) (< (`self.Apply Chain Index`) (`self.Maximum Chain Length`)))
              (if (< _apply_chain_index (`self.Current Chain Length`))
                (`SceneComponent.K2_SetRelativeTransform` (`|GetArrayItem` (`self.Chain Pieces`) (`self.Apply Chain Index`)) _returnvalue_4 false false)
                (else
                  (bind _returnvalue_5 (`AddComponent|NODE_AddStaticMeshComponent-2` :`RelativeTransform` _returnvalue_4))
                  (`StaticMeshComponent.SetStaticMesh` _returnvalue_5 _static_mesh)
                  (`PrimitiveComponent.SetMaterial` _returnvalue_5 0 (`self.Pickaxe Material`))
                  (`PrimitiveComponent.SetCollisionEnabled` _returnvalue_5 "NoCollision")
                  (`KismetArrayLibrary.Array_Add` (`self.Chain Pieces`) _returnvalue_5)
                  (`/Engine/EditorBlueprintResources/StandardMacros.IncrementInt` (`self.Current Chain Length`)
                    (:`  `
                      _))))
              (bind _output_get (set `self.Apply Chain Distance` (- (stale _output_get) _skip)))
              (`/Engine/EditorBlueprintResources/StandardMacros.IncrementInt` (`self.Apply Chain Index`))))
          (:`then_1`
            (`SceneComponent.K2_SetWorldLocation` (`self.Grabber`) (`self.Current Location`) false false)))))))

(fn `Attach To Hand`
  (bind (_drg_context_drgcontextavailable _drg_context_drgperkasset _drg_context_drgplayercharacter) (break `/Game/ClawPerk/F_DrgContext` (`self.DRG Context`)))
  (bind _fpmesh (`PlayerCharacter.FPMesh` _drg_context_drgplayercharacter))
  (bind _returnvalue_location (`KismetMathLibrary.BreakTransform` (`SceneComponent.GetSocketTransform` _fpmesh "Dwarf_HandL_Attach" "RTS_ParentBoneSpace")))
  (if _drg_context_drgcontextavailable
    (`self.K2_AttachToComponent` _fpmesh "Dwarf_HandL_Attach" "KeepRelative" "KeepRelative" "KeepRelative")
    (`self.K2_SetActorRelativeTransform` (`KismetMathLibrary.MakeTransform` (* _returnvalue_location (-2.0 -2.0 1.0))))))

(fn `Fire`
  (set `self.State` "NewEnumerator0")
  (`SkeletalMeshComponent.PlayAnimation` (`self.Grabber`) "/Game/ClawPerk/ClawAsset/Grabber_Anim_Approach.Grabber_Anim_Approach" true))

(fn `Game Initialize`
  (params (`Make Hook Args` :type "/Game/ClawPerk/F_MakeHookArgs Structure"))
  (bind (_target _targetposition _targetinfo _drgcontext) (break `/Game/ClawPerk/F_MakeHookArgs` `Make Hook Args`))
  (set `self.Target Actor` _target)
  (set `self.Target Actor Info` _targetinfo)
  (set `self.DRG Context` _drgcontext)
  (set `self.Target Relative To Actor` (- _targetposition (`self.K2_GetActorLocation` _target)))
  (`self.Make Hook`)
  (`self.Attach To Hand`)
  (set `self.Attach Location` (.location (`SceneComponent.GetRelativeTransform` (`self.Grabber`)))) ; Save the claw's initial position.
  (set `self.Current Location` (`self.Source Location`)) ; Initialize current position.
)

(fn `Get Chain Link From Index`
  (params (Index :type Integer))
  (returns (`Instance Static Mesh Component` :type "InstancedStaticMeshComponent Object Reference") (`Out Index` :type Integer) (`Origin Offset` :type "Float (double-precision)") (Length :type "Float (double-precision)") (Skip :type "Float (double-precision)") (`Debug Name` :type String) (`Static Mesh` :type "StaticMesh Object Reference"))
  (locals (`Chosen Component` :type "InstancedStaticMeshComponent Object Reference") (`Chosen Offset` :type "Float (double-precision)") (`Chosen Length` :type "Float (double-precision)") (`Chosen Skip` :type "Float (double-precision)") (`Chosen Name` :type String) (`Chosen Mesh` :type "StaticMesh Object Reference"))
  (switch `int` (mod Index 2)
    (:`0`
      (set `local.Chosen Component` (`self.Instanced Handles`))
      (set `local.Chosen Offset` (`self.Handle Origin Offset`))
      (set `local.Chosen Length` (`self.Handle Length`))
      (set `local.Chosen Skip` (`self.Handle Skip`))
      (set `local.Chosen Name` "Handle")
      (set `local.Chosen Mesh` (`self.Handle Mesh`)))
    (:`1`
      (set `local.Chosen Component` (`self.Instanced Heads`))
      (set `local.Chosen Offset` (`self.Head Origin Offset`))
      (set `local.Chosen Length` (`self.Head Length`))
      (set `local.Chosen Skip` (`self.Head Skip`))
      (set `local.Chosen Name` "Head")
      (set `local.Chosen Mesh` (`self.Head Mesh`))))
  (return (`local.Chosen Component`) (/ Index 2) (`local.Chosen Offset`) (`local.Chosen Length`) (`local.Chosen Skip`) "Handle" (`local.Chosen Mesh`)))

(fn `Grab Target`
  (bind _target_actor (`self.Target Actor`))
  (bind (_type _pathfindercharacter) (break `/Game/ClawPerk/F_GrabbedObjectInfo` (`self.Target Actor Info`)))
  (set `self.Is Actor Grabbed` true)
  (set `self.Grabbed Actor` _target_actor)
  (`self.Log` (`KismetStringLibrary.Concat_StrStr` "Grabbed " (`KismetSystemLibrary.GetDisplayName` _target_actor) "!"))
  (switch `/Game/ClawPerk/E_GrabbedObjectType` _type
    (:`NewEnumerator1`
      (`DeepPathfinderMovement.SetControlledExternally` (`DeepPathfinderCharacter.PathfinderMovement` _pathfindercharacter) true))))

(fn `Init Spline`
  (params (`Number of points` :type Integer))
  (locals (points :type "Array of Vector Structure"))
  (for _index (range (+ `Number of points` 1))
    (`KismetArrayLibrary.Array_Add` (`local.points`) (`KismetMathLibrary.MakeVector` (`KismetMathLibrary.Conv_IntToDouble` _index)))
    (`KismetArrayLibrary.Array_Add` (`self.Hook Recoil Offsets`)))
  (`SplineComponent.SetSplinePoints` (`self.Spline`) (`local.points`) "Local" true))

(fn `Is destination reached`
  (returns (`Is Reached` :type Boolean))
  (return (< (`KismetMathLibrary.Vector_Distance` (`self.Current Location`) (`self.Target Location`)) (`self.Distance Tolerance`))))

(fn `Log`
  (params (`Log Entry` :type String))
  (bind _drglib (`self.DRGLib`))
  (`/Engine/EditorBlueprintResources/StandardMacros.IsValid` _drglib
    (:`Is Valid`
      (`/Game/DRGLib/LoggingFunctions/LIB_F_Log.AddLogEntry` _drglib "NewEnumerator2" "Hook" `Log Entry`))
    (:`Is Not Valid`
      (`KismetSystemLibrary.PrintString` `Log Entry`))))

(fn `Make Hook`
  (bind (_drg_context_drgcontextavailable _drg_context_drgperkasset _drg_context_drgplayercharacter) (break `/Game/ClawPerk/F_DrgContext` (`self.DRG Context`)))
  (if _drg_context_drgcontextavailable
    (bind (_parts_to_static_mesh _material) (`/Game/ClawPerk/BP_ClawFunctionLibrary.Get Player Character Pieces` _drg_context_drgplayercharacter))
    (`self.Make Hook With Parts` _parts_to_static_mesh _material)
    (else
      (`self.Make Hook With Parts` (`|MakeMap` "Head" "/Game/ClawPerk/TestAssets/drg_hook_SM_Pickaxe_Head_ArcWelders_S01_mo.drg_hook_SM_Pickaxe_Head_ArcWelders_S01_mo" "Shaft" "/Game/ClawPerk/TestAssets/drg_hook_SM_PickAxe_Shaft_009_mo.drg_hook_SM_PickAxe_Shaft_009_mo" "FrontBlade" "/Game/ClawPerk/TestAssets/drg_hook_SM_PickAxe_BladeFront_005_mo.drg_hook_SM_PickAxe_BladeFront_005_mo" "BackBlade" "/Game/ClawPerk/TestAssets/drg_hook_SM_PickAxe_BladeSpecial_Chasmborne_mo.drg_hook_SM_PickAxe_BladeSpecial_Chasmborne_mo" "Handle" "/Game/ClawPerk/TestAssets/drg_hook_SM_PickAxe_Handle_ReapersClaw_mo.drg_hook_SM_PickAxe_Handle_ReapersClaw_mo" "Pommel" "/Game/ClawPerk/TestAssets/drg_hook_SM_PickAxe_Pommel_ReapersClaw_mo.drg_hook_SM_PickAxe_Pommel_ReapersClaw_mo" :!type "EPickaxePartLocation Enum" :!valuetype "StaticMesh Object Reference")))))

(fn `Make Hook With Parts`
  (params (`Part To Mesh` :type "Map of EPickaxePartLocation Enum to StaticMesh Object Reference") (Material :type "MaterialInterface Object Reference"))
  (bind _shaft_relative_transform (`self.Shaft Relative Transform`))
  (bind _blade_relative_transform (`self.Blade Relative Transform`))
  (bind _instanced_handles (`self.Instanced Handles`))
  (bind _instanced_heads (`self.Instanced Heads`))
  (bind _material (`local.Material`))
  (bind _part_to_mesh (`local.Part To Mesh`))
  (`self.Make Pieces` `Part To Mesh` Material (`self.Grabber`) (`|MakeArray` (make `/Game/ClawPerk/F_ClawPiece` "Head" "Bone-Base" (`self.Head Relative Transform`)) (make `/Game/ClawPerk/F_ClawPiece` "Shaft" "Bone-Front-Shaft" _shaft_relative_transform) (make `/Game/ClawPerk/F_ClawPiece` "Shaft" "Bone-Special-Shaft" (`KismetMathLibrary.ComposeTransforms` _shaft_relative_transform (`KismetMathLibrary.MakeTransform` (0.0 0.0 0.0)))) (make `/Game/ClawPerk/F_ClawPiece` "FrontBlade" "Bone-Front" _blade_relative_transform) (make `/Game/ClawPerk/F_ClawPiece` "BackBlade" "Bone-Special" (`KismetMathLibrary.ComposeTransforms` _blade_relative_transform (`KismetMathLibrary.MakeTransform` (0.0 0.0 0.0) (struct :`Pitch` 180.0)))))) ; Create the claw
  (`self.Make Pieces` `Part To Mesh` Material (`self.Handle`) (`|MakeArray` (make `/Game/ClawPerk/F_ClawPiece` "Handle" "None" (`self.RT Grabber Handle`)) (make `/Game/ClawPerk/F_ClawPiece` "Shaft" "None" (`self.RT Grabber Shaft`)) (make `/Game/ClawPerk/F_ClawPiece` "Pommel" "None" (`self.RT Grabber Pommel`)) (make `/Game/ClawPerk/F_ClawPiece` "Head" "None" (`self.RT Grabber Head`)))) ; Create the handle
  (bind _output_get (set `self.Handle Mesh` (`BlueprintMapLibrary.Map_Find` _part_to_mesh "Handle")))
  (`StaticMeshComponent.SetStaticMesh` _instanced_handles _output_get)
  (`PrimitiveComponent.SetMaterial` _instanced_handles 0 _material)
  (bind _output_get_2 (set `self.Head Mesh` (`BlueprintMapLibrary.Map_Find` _part_to_mesh "Head")))
  (`StaticMeshComponent.SetStaticMesh` _instanced_heads _output_get_2)
  (`PrimitiveComponent.SetMaterial` _instanced_heads 0 _material)
  (set `self.Pickaxe Material` _material))

(fn `Make Pieces`
  (params (`Part To Mesh` :type "Map of EPickaxePartLocation Enum to StaticMesh Object Reference") (Material :type "MaterialInterface Object Reference") (`Scene Component` :type "SceneComponent Object Reference") (Pieces :type "Array of /Game/ClawPerk/F_ClawPiece Structure"))
  (for _array_element Pieces
    (bind (_partlocation _bonename _relativetransform) (break `/Game/ClawPerk/F_ClawPiece` _array_element))
    (if (or (== _bonename "None") (`SceneComponent.DoesSocketExist` (`local.Scene Component`) _bonename))
      (bind _returnvalue (`AddComponent|NODE_AddStaticMeshComponent-4` :`bManualAttachment` true :`RelativeTransform` (`KismetMathLibrary.MakeTransform` (.location _relativetransform) (.rotation _relativetransform) (* (.scale _relativetransform) (`SceneComponent.K2_GetComponentScale` (`local.Scene Component`))))))
      (`StaticMeshComponent.SetStaticMesh` _returnvalue (`BlueprintMapLibrary.Map_Find` (`local.Part To Mesh`) _partlocation))
      (`PrimitiveComponent.SetMaterial` _returnvalue 0 (`local.Material`))
      (`PrimitiveComponent.SetCollisionEnabled` _returnvalue "NoCollision")
      (`SceneComponent.K2_AttachToComponent` _returnvalue (`local.Scene Component`) _bonename "KeepRelative" "KeepRelative" "KeepWorld" false)
      (else
        (`KismetSystemLibrary.PrintString` (`KismetStringLibrary.Concat_StrStr` "The bone " (`KismetStringLibrary.Conv_NameToString` _bonename) " does not exist."))))))

(fn `Release Target`
  (bind (_drg_context_drgcontextavailable _drg_context_drgperkasset _drg_context_drgplayercharacter) (break `/Game/ClawPerk/F_DrgContext` (`self.DRG Context`)))
  (bind (_drg_context_drgcontextavailable_2 _drg_context_drgperkasset_2 _drg_context_drgplayercharacter_2) (break `/Game/ClawPerk/F_DrgContext` (`self.DRG Context`)))
  (bind (_type _pathfindercharacter _collectiblebase _carriablecomponent _usablecomponent) (break `/Game/ClawPerk/F_GrabbedObjectInfo` (`self.Target Actor Info`)))
  (if (`self.Is Actor Grabbed`)
    (set `self.Is Actor Grabbed` false) ; Grabbed actor is no longer valid.
    (if _drg_context_drgcontextavailable_2
      (switch `/Game/ClawPerk/E_GrabbedObjectType` _type
        (:`NewEnumerator0`
          (`self.K2_SetActorRotation` (`self.Target Actor`) (`KismetMathLibrary.MakeRotator` 0.0 0.0 (.yaw (`PlayerCharacter.GetAimRotation` _drg_context_drgplayercharacter_2))) false))
        (:`NewEnumerator1`
          (`DeepPathfinderMovement.SetControlledExternally` (`DeepPathfinderCharacter.PathfinderMovement` _pathfindercharacter) false))
        (:`NewEnumerator2`
          (`UsableComponentBase.BeginUse` (`/Game/GameElements/Resources/Collectibles/BP_Collectible_Base.InstantUsable` _collectiblebase) _drg_context_drgplayercharacter "Use"))
        (:`NewEnumerator3`
          (`CarriableComponent.PickupItem` _carriablecomponent _drg_context_drgplayercharacter))
        (:`NewEnumerator5`
          (`SingleUsableComponent.Use` _usablecomponent _drg_context_drgplayercharacter "Use" 1.0)
          (`UsableComponentBase.BeginUse` (`self.Fake Usable`) _drg_context_drgplayercharacter "Use")))
      (`PerkAsset.UseCharge` _drg_context_drgperkasset (`PlayerCharacter.GetPlayerController` _drg_context_drgplayercharacter)))))

(fn `Source Location`
  (returns (Source :type "Vector Structure"))
  (return (`FSDConversionLibrary.ComponentToWorldLocation` (`self.Attach Point`))))

(fn `Target Location`
  (returns (Destination :type "Vector Structure"))
  (bind _target_actor (`self.Target Actor`))
  (switch `/Game/ClawPerk/E_ClawState` (`self.State`)
    (:`NewEnumerator0`
      (`/Engine/EditorBlueprintResources/StandardMacros.IsValid` _target_actor :!label _label
        (:`Is Valid`
          _)
        (:`Is Not Valid`
          (return (`self.Source Location`)))))
    (:`NewEnumerator1`
      (goto _label))
    (:`NewEnumerator2`
      (return (`self.Source Location`)))
    (:`NewEnumerator3`
      (return (`self.Source Location`))))
  (return (+ (`self.K2_GetActorLocation` _target_actor) (`self.Target Relative To Actor`))))

(fn `Update Grabbed Target`
  (bind _grabbed_actor (`self.Grabbed Actor`))
  (bind _returnvalue (- (`self.Current Location`) (`self.Target Relative To Actor`)))
  (`/Engine/EditorBlueprintResources/ActorMacros.Switch Has Authority` ; Only run on server.
    (:`Authority`
      (if (`self.Is Actor Grabbed`)
        (`/Engine/EditorBlueprintResources/StandardMacros.IsValid` _grabbed_actor ; Make sure the grabbed actor is still valid.
          (:`Is Valid`
            (switch `/Game/ClawPerk/E_GrabbedObjectType` (`.Type_14_7B5B80B343C99BDA4E6C0DBD5E3A0210` (break `/Game/ClawPerk/F_GrabbedObjectInfo` (`self.Target Actor Info`)))
              (:`NewEnumerator0`
                _)
              (:`NewEnumerator1`
                _)
              (:`NewEnumerator2`
                _)
              (:`NewEnumerator3`
                _)
              (:`NewEnumerator5`
                _))
            (bind _sweephitresult (`self.K2_SetActorLocation` _grabbed_actor _returnvalue true false)) ; Update actor position.
            (if (or (`GameplayStatics.BreakHitResult` _sweephitresult) (< (`KismetMathLibrary.Vector_Distance` _returnvalue (`self.Source Location`)) 200.0))
              (`self.Release Target`)))
          (:`Is Not Valid`
            (set `self.Is Actor Grabbed` false) ; Grabbed actor is no longer valid.
          ))))))

(fn `Update Spline Points`
  (params (`Delta Seconds` :type "Float (double-precision)"))
  (bind _source (`self.Source Location`))
  (bind _destination (`self.Target Location`))
  (bind _current_location (`self.Current Location`))
  (bind _spline (`self.Spline`))
  (bind _returnvalue (`SplineComponent.GetNumberOfSplinePoints` (`self.Spline`)))
  (bind _output_get (set `self.Current Location` (+ (stale _output_get) (* (`KismetMathLibrary.GetDirectionUnitVector` _current_location _destination) (`KismetMathLibrary.FMin` (`KismetMathLibrary.Vector_Distance` _current_location _destination) (* (`self.Distance Per Second`) `Delta Seconds`))))))
  (for _index (range _returnvalue)
    (`SplineComponent.SetLocationAtSplinePoint` _spline _index (+ (* (- (`self.Current Location`) _source) (/ (`KismetMathLibrary.Conv_IntToDouble` _index) (`KismetMathLibrary.Conv_IntToDouble` _returnvalue))) _source (`|GetArrayItem` (`self.Hook Recoil Offsets`) _index)) "World" false))
  (`SplineComponent.UpdateSpline` _spline))

(fn `UserConstructionScript`
  (if (not (`KismetSystemLibrary.IsPackagedForDistribution`))
    (`self.Make Hook With Parts` (`|MakeMap` "Head" "/Game/ClawPerk/TestAssets/drg_hook_SM_Pickaxe_Head_ArcWelders_S01_mo.drg_hook_SM_Pickaxe_Head_ArcWelders_S01_mo" "Shaft" "/Game/ClawPerk/TestAssets/drg_hook_SM_PickAxe_Shaft_009_mo.drg_hook_SM_PickAxe_Shaft_009_mo" "FrontBlade" "/Game/ClawPerk/TestAssets/drg_hook_SM_PickAxe_BladeFront_005_mo.drg_hook_SM_PickAxe_BladeFront_005_mo" "BackBlade" "/Game/ClawPerk/TestAssets/drg_hook_SM_PickAxe_BladeSpecial_Chasmborne_mo.drg_hook_SM_PickAxe_BladeSpecial_Chasmborne_mo" "Handle" "/Game/ClawPerk/TestAssets/drg_hook_SM_PickAxe_Handle_ReapersClaw_mo.drg_hook_SM_PickAxe_Handle_ReapersClaw_mo" "Pommel" "/Game/ClawPerk/TestAssets/drg_hook_SM_PickAxe_Pommel_ReapersClaw_mo.drg_hook_SM_PickAxe_Pommel_ReapersClaw_mo" :!type "EPickaxePartLocation Enum" :!valuetype "StaticMesh Object Reference"))))