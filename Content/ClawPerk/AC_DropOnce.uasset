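; One-shot actor component that drops its owner onto the terrain, then destroys itself.
; On BeginPlay it reuses or adds DropToTerrain and TerrainDetect components, links the detector as the terrain point and begins drop detection.
; A Flip latch waits for a fall to start and end, then conditionally stops drop detection before self-destruction.
; The stop flag for terrain detection is set, but its branch is empty.
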(event `self.ReceiveBeginPlay`
  (bind _returnvalue (`self.GetOwner`))
  (bind _returnvalue_2 (`self.GetOwner`))
  (bind _drop_to_terrain_component (`self.Drop To Terrain Component`))
  (bind _terrain_detect_component (`self.Terrain Detect Component`))
  (`|ExecutionSequence`
    (:`then_0`
      (bind _returnvalue_3 (`ActorFunctionLibrary.GetComponentByClass` _returnvalue_2 "/Script/FSD.DropToTerrainComponent"))
      (bind _asdrop_to_terrain_component (cast `DropToTerrainComponent` _returnvalue_3)
        (:`then`
          (set `self.Drop To Terrain Component` _asdrop_to_terrain_component)
          (set `self.Stop Drop Component When Completed` false))
        (:`CastFailed`
          (bind _returnvalue_4 (`|AddComponentByClass` _returnvalue "/Script/FSD.DropToTerrainComponent"))
          (bind _output_get (set `self.Drop To Terrain Component` _returnvalue_4))
          (set `self.Stop Drop Component When Completed` (`DropToTerrainComponent.IsDetecting` _output_get)))))
    (:`then_1`
      (bind _returnvalue_5 (`ActorFunctionLibrary.GetComponentByClass` _returnvalue_2 "/Script/FSD.TerrainDetectComponent"))
      (bind _asterrain_detect_component (cast `TerrainDetectComponent` _returnvalue_5)
        (:`then`
          (set `self.Terrain Detect Component` _asterrain_detect_component)
          (set `self.Stop Terrain Detect Component When Completed` false))
        (:`CastFailed`
          (bind _returnvalue_6 (`|AddComponentByClass` _returnvalue "/Script/FSD.TerrainDetectComponent" false (`KismetMathLibrary.MakeTransform` (0.0 0.0 -1.0))))
          (set `self.Terrain Detect Component` _returnvalue_6)
          (set `self.Stop Terrain Detect Component When Completed` true))))
    (:`then_2`
      (`TerrainDetectComponent.StartDetect` _terrain_detect_component)
      (add `DropToTerrainComponent.OnFallToTerrainStateChanged` _drop_to_terrain_component (delegate `Is falling`))
      (set `DropToTerrainComponent.TerrainPoints` (`|MakeArray` _terrain_detect_component) _drop_to_terrain_component)
      (set `DropToTerrainComponent.FallVelocity` 500.0 _drop_to_terrain_component)
      (`DropToTerrainComponent.BeginDropDetection` _drop_to_terrain_component))))

(event `Is falling`
  (params (IsFalling :type Boolean))
  (bind _flip (`self.Flip`))
  (if (and IsFalling (not _flip))
    (set `self.Flip` true)
    (elif (and (not IsFalling) _flip)
      (`|ExecutionSequence`
        (:`then_0`
          (if (`self.Stop Drop Component When Completed`)
            (`DropToTerrainComponent.StopDropDetection` (`self.Drop To Terrain Component`) false)))
        (:`then_1`
          (if (`self.Stop Terrain Detect Component When Completed`)
            _))
        (:`then_2`
          (`self.K2_DestroyComponent`))))))