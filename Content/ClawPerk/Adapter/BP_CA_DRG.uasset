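; Adapter that connects the claw perk's BPClaw to the DRG player character, perk asset and controller.
; Setup copies the equipped pickaxe's part meshes and material into the claw's hook, then attaches the claw to the first-person left-hand socket with a socket-derived offset.
; Events forward collectible, carriable and detonation pack pickups and charge use to the game's objects.
; Drop rotation follows only the player's aim yaw.
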(event `/Game/ClawPerk/Adapter/BI_ClawAdapter.Setup`
  (params (BP_Claw :type "/Game/ClawPerk/BP_Claw Object Reference"))
  (bind _bp_claw (`self.BP_Claw`))
  (bind _pickaxe_parts_to_static_mesh (`self.Pickaxe Parts To Static Mesh`))
  (bind _fpmesh (`PlayerCharacter.FPMesh` (`self.Player Character`)))
  (bind _returnvalue_location (`KismetMathLibrary.BreakTransform` (`SceneComponent.GetSocketTransform` _fpmesh "Dwarf_HandL_Attach" "RTS_ParentBoneSpace")))
  (bind _miningitem (`InventoryComponent.MiningItem` (`PlayerCharacter.InventoryComponent` (`self.Player Character`))))
  (bind _equippedparts (`PickaxeItem.EquippedParts` _miningitem))
  (set `self.BP_Claw` BP_Claw)
  (`|ExecutionSequence`
    (:`then_0`
      ;[1 0.05729 0.05729] Extract pickaxe part meshes from PlayerCharacter->InventoryComponent->MiningItem->EquippedParts and send it to Make Hook.
      (set `self.Pickaxe Parts To Static Mesh` (`|MakeMap`))
      (bind _keys (`BlueprintMapLibrary.Map_Keys` _equippedparts))
      (bind _values (`BlueprintMapLibrary.Map_Values` _equippedparts))
      (for (_array_element _array_index) _keys
        (bind _asstatic_mesh_component (cast `StaticMeshComponent` (`.TP_Mesh` (break `PickaxeMeshInstance` (`|GetArrayItem` _values _array_index)))))
        (`BlueprintMapLibrary.Map_Add` _pickaxe_parts_to_static_mesh _array_element (`StaticMeshComponent.StaticMesh` _asstatic_mesh_component)))
      (`/Game/ClawPerk/BP_Claw.Make Hook With Parts` (`self.BP_Claw`) _pickaxe_parts_to_static_mesh (`PickaxeItem.EquippedMaterial` _miningitem)))
    (:`then_1`
      ;[0.308 0.519 1] Attach to hand
      (`Actor.K2_AttachToComponent` _bp_claw _fpmesh "Dwarf_HandL_Attach" "KeepRelative" "KeepRelative" "KeepRelative" true)
      (`Actor.K2_SetActorRelativeTransform` _bp_claw (`KismetMathLibrary.MakeTransform` (* _returnvalue_location (-2.0 -2.0 1.0))) false false))))

(event `/Game/ClawPerk/Adapter/BI_ClawAdapter.Pick up Collectible`
  (params (`Instant Usable` :type "InstantUsable Object Reference"))
  (`UsableComponentBase.BeginUse` `Instant Usable` (`self.Player Character`) "Use"))

(event `/Game/ClawPerk/Adapter/BI_ClawAdapter.Pick up Carriable`
  (params (`Carriable Component` :type "CarriableComponent Object Reference"))
  (`CarriableComponent.PickupItem` `Carriable Component` (`self.Player Character`)))

(event `/Game/ClawPerk/Adapter/BI_ClawAdapter.Pick up Detonation Pack`
  (params (`Single Usable Component` :type "SingleUsableComponent Object Reference") (`Fake Usable` :type "InstantUsable Object Reference"))
  (bind _player_character (`self.Player Character`))
  (`SingleUsableComponent.Use` `Single Usable Component` _player_character "Use" 1.0)
  (`UsableComponentBase.BeginUse` `Fake Usable` _player_character "Use"))

(event `/Game/ClawPerk/Adapter/BI_ClawAdapter.Use Charge`
  (`PerkAsset.UseCharge` (`self.Perk Asset`) (`self.Player Controller`)))

(fn `Construct`
  (params (`Player Character` :type "PlayerCharacter Object Reference") (`Perk Asset` :type "PerkAsset Object Reference") (`Player Controller` :type "PlayerController Object Reference"))
  (set `self.Player Character` `Player Character`)
  (set `self.Perk Asset` `Perk Asset`)
  (set `self.Player Controller` `Player Controller`))

(fn `Get Drop Rotation`
  (returns (Rotation :type "Rotator Structure"))
  (return (`KismetMathLibrary.MakeRotator` 0.0 0.0 (.yaw (`PlayerCharacter.GetAimRotation` (`self.Player Character`))))))