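; Claw hook projectile for a Deep Rock Galactic perk mod that pulls a target back to the player, built from pickaxe parts.
; Tick moves it toward the target, grabs, then retracts to a drop point before the player, carrying grabbable actors along.
; Multicasts share state, while the visible grabber blends between handle attach point and true position.
; On release, the server spends a perk charge, triggers type-specific pickup or use, and destroys the handle.
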(event `self.ReceiveBeginPlay`
  ;[1 0.04062 0.04062] Begin Play
  (`/Game/ClawPerk/BP_ClawFunctionLibrary.Make Pieces from DRG Context` (`.DRGContext_23_E46872554C41985D51C363B53E8BAA09` (break `/Game/ClawPerk/F_MakeHookArgs` (`self.Make Hook Args`))) (`self.Grabber`) (`self.Get Model Pieces`) (`/Game/ClawPerk/BP_ClawFunctionLibrary.Get Editor Pickaxe Part Testing Array`)))

(event `self.ReceiveTick`
  (params (DeltaSeconds :type "Float (single-precision)"))
  (bind _target_location (`self.Target Location`))
  (bind _returnvalue (`self.K2_GetActorLocation`))
  (bind _grabber (`self.Grabber`))
  (bind _handle (`self.Handle`))
  (bind _returnvalue_2 (`KismetMathLibrary.Vector_Distance` _returnvalue _target_location))
  (bind _attach_point (`/Game/ClawPerk/BP_Claw.Attach Point` _handle))
  ;[1 0 0.008587] Event Tick
  (`|ExecutionSequence`
    (:`then_0`
      ;;[1 0.2542 0.6504] Update location
      (`/Engine/EditorBlueprintResources/StandardMacros.IsValid` (`self.Handle`)
        (:`Is Valid`
          (`self.K2_SetActorLocation` (+ _returnvalue (* (`KismetMathLibrary.GetDirectionUnitVector` _returnvalue _target_location) (`KismetMathLibrary.FMin` _returnvalue_2 (* (`self.Distance Per Second`) DeltaSeconds)))))
          ;;;[0.6653 1 0.2509] On Destination reached
          (if (< _returnvalue_2 (`self.Distance Tolerance`))
            (switch `/Game/ClawPerk/E_ClawState` (`self.Claw State`)
              (:`NewEnumerator0`
                (`self.Grab Target`)
                (`self.Retract Multicast`))
              (:`NewEnumerator2`
                (`self.Release Target`)))))))
    (:`then_1`
      (if (not (`self.IsActorBeingDestroyed`))
        (`|ExecutionSequence`
          (:`then_0`
            ;;[1 0.4641 0.1309] Client hook position > server position
            (if (not (== (`self.Claw State`) (enumliteral `/Game/ClawPerk/E_ClawState` "NewEnumerator3")))
              (bind (_direction _lerp_between_client_and_true_position) (`Timeline|luna tuna`)
                (:`Update`
                  (set `self.Attach Point to Real Point lerp` _lerp_between_client_and_true_position)))))
          (:`then_1`
            ;;;[1 0.1789 0.562] Lerp between client attach point and real point
            (`/Engine/EditorBlueprintResources/StandardMacros.IsValid` _handle ; Ensure the handle is still valid.\nTODO: It may be a good idea to set the grabber's\nlocation to the actor's location when the handle no\nlonger exists.
              (:`Is Valid`
                (`SceneComponent.K2_SetWorldLocation` _grabber (`KismetMathLibrary.VLerp` (`SceneComponent.K2_GetComponentLocation` _attach_point) (`self.K2_GetActorLocation`) (`self.Attach Point to Real Point lerp`)) false false)
                (if (`|EnumEquality` (`self.Claw State`) "NewEnumerator3")
                  (`SceneComponent.K2_SetWorldRotation` _grabber (`SceneComponent.K2_GetComponentRotation` _attach_point) false false)))))
          (:`then_2`
            (`self.Update Grabbed Target`)))))))

(event `Fire Multicast`
  ;[1 0.1432 0.7478] Fire (Multicast)
  (set `self.Claw State` "NewEnumerator0")
  (`self.Update Rotation`))

(event `Fire Server`
  ;[1 0.3862 0.003982] Fire (Server)
  (`self.Fire Multicast`))

(event `Grab Multicast`
  (params (`Was Grabbed` :type Boolean))
  ;[1 0.1949 0.8564] On Grab (Multicast)
  (set `self.Is Actor Grabbed` `Was Grabbed`))

(event `Retract Multicast`
  ;[1 0.2581 0.7427] Retract (Multicast)
  (set `self.Claw State` "NewEnumerator2"))

(event `Release Actor Multicast`
  (bind ((`TargetInfo_11_8C569593462C5C3571677DABECAC2508` _targetinfo) (`DRGContext_23_E46872554C41985D51C363B53E8BAA09` _drgcontext)) (break `/Game/ClawPerk/F_MakeHookArgs` (`self.Make Hook Args`)))
  (bind ((`Type_14_7B5B80B343C99BDA4E6C0DBD5E3A0210` _type) (`CollectibleBase_11_74E9D1714E7BF2CDEC71368D4724A985` _collectiblebase) (`CarriableComponent_6_1B3B74D546E577A40FD1DDBC77F5E328` _carriablecomponent) (`UsableComponent_17_0CAA5EFE47645D7BC28A96A332A2E1E6` _usablecomponent)) (break `/Game/ClawPerk/F_GrabbedObjectInfo` _targetinfo))
  (bind (_drgcontextavailable _drgperkasset _drgplayercharacter) (break `/Game/ClawPerk/F_DrgContext` _drgcontext))
  ;[1 0.3515 0.9126] Release Actor (Multicast)
  (if _drgcontextavailable
    (switch `/Game/ClawPerk/E_GrabbedObjectType` _type
      (:`NewEnumerator2`
        (`UsableComponentBase.BeginUse` (`/Game/GameElements/Resources/Collectibles/BP_Collectible_Base.InstantUsable` _collectiblebase) _drgplayercharacter "Use"))
      (:`NewEnumerator3`
        (`CarriableComponent.PickupItem` _carriablecomponent _drgplayercharacter))
      (:`NewEnumerator5`
        (`SingleUsableComponent.Use` _usablecomponent _drgplayercharacter "Use" 1.0)
        (`UsableComponentBase.BeginUse` (`self.Fake Usable`) _drgplayercharacter "Use")))))

(fn `Get Drop Point`
  (returns (`Drop Location` :type "Vector Structure"))
  (bind _handle (`self.Handle`))
  (bind ((`DRGContextAvailable_1_D205758E44DE73B207E34EB032FC3D06` _drgcontextavailable) (`DRGPlayerCharacter_7_C22F1CB1404240AA94A275ABA95557C7` _drgplayercharacter)) (break `/Game/ClawPerk/F_DrgContext` (`.DRGContext_23_E46872554C41985D51C363B53E8BAA09` (break `/Game/ClawPerk/F_MakeHookArgs` (`self.Make Hook Args`)))))
  (if _drgcontextavailable
    (return (+ (* (`KismetMathLibrary.GetForwardVector` (`PlayerCharacter.GetAimRotation` _drgplayercharacter)) 100.0) (`SceneComponent.K2_GetComponentLocation` (`PlayerCharacter.FirstPersonRoot` _drgplayercharacter))))
    (else
      (return (+ (`self.K2_GetActorLocation` _handle) (* (`KismetMathLibrary.GetForwardVector` (`self.K2_GetActorRotation` _handle)) 100.0))))))

(fn `Get Model Pieces`
  (returns (`Claw Pieces` :type "Array of /Game/ClawPerk/F_ClawPiece Structure"))
  (bind _shaft_relative_transform (`self.Shaft Relative Transform`))
  (bind _blade_relative_transform (`self.Blade Relative Transform`))
  (return (`|MakeArray` (make `/Game/ClawPerk/F_ClawPiece` "Head" "Bone-Base" (`self.Head Relative Transform`)) (make `/Game/ClawPerk/F_ClawPiece` "Shaft" "Bone-Front-Shaft" _shaft_relative_transform) (make `/Game/ClawPerk/F_ClawPiece` "Shaft" "Bone-Special-Shaft" (`KismetMathLibrary.ComposeTransforms` _shaft_relative_transform (`KismetMathLibrary.MakeTransform` (0.0 0.0 0.0)))) (make `/Game/ClawPerk/F_ClawPiece` "FrontBlade" "Bone-Front" _blade_relative_transform) (make `/Game/ClawPerk/F_ClawPiece` "BackBlade" "Bone-Special" (`KismetMathLibrary.ComposeTransforms` _blade_relative_transform (`KismetMathLibrary.MakeTransform` (0.0 0.0 0.0) (struct :`Pitch` 180.0)))))))

(fn `Grab Target`
  (bind ((`Type_14_7B5B80B343C99BDA4E6C0DBD5E3A0210` _type) (`PathfinderCharacter_2_25853F2D40E1B0E7C83EB18A9FC05298` _pathfindercharacter)) (break `/Game/ClawPerk/F_GrabbedObjectInfo` (`.TargetInfo_11_8C569593462C5C3571677DABECAC2508` (break `/Game/ClawPerk/F_MakeHookArgs` (`self.Make Hook Args`)))))
  (bind _output_get (set `self.Is Actor Grabbed` (`|EnumInequality` _type (enumliteral `/Game/ClawPerk/E_GrabbedObjectType` "NewEnumerator4"))))
  (`self.Grab Multicast` _output_get)
  (if _output_get
    (switch `/Game/ClawPerk/E_GrabbedObjectType` _type
      (:`NewEnumerator1`
        (`DeepPathfinderMovement.SetControlledExternally` (`DeepPathfinderCharacter.PathfinderMovement` _pathfindercharacter) true) ; Allows us to move pathfinder characters
      ))))

(fn `Release Target`
  (bind ((`Target_5_63C167034DFEE7C34BA8FFB2C364DDC8` _target) (`TargetInfo_11_8C569593462C5C3571677DABECAC2508` _targetinfo) (`DRGContext_23_E46872554C41985D51C363B53E8BAA09` _drgcontext)) (break `/Game/ClawPerk/F_MakeHookArgs` (`self.Make Hook Args`)))
  (bind (_drgcontextavailable _drgperkasset _drgplayercharacter) (break `/Game/ClawPerk/F_DrgContext` _drgcontext))
  (bind ((`Type_14_7B5B80B343C99BDA4E6C0DBD5E3A0210` _type) (`PathfinderCharacter_2_25853F2D40E1B0E7C83EB18A9FC05298` _pathfindercharacter)) (break `/Game/ClawPerk/F_GrabbedObjectInfo` _targetinfo))
  (if (`self.Is Actor Grabbed`)
    (set `self.Is Actor Grabbed` false)
    (`/Engine/EditorBlueprintResources/ActorMacros.Switch Has Authority`
      (:`Authority`
        (`|ExecutionSequence`
          (:`then_0`
            (if _drgcontextavailable
              (`PerkAsset.UseCharge` _drgperkasset (`PlayerCharacter.GetPlayerController` _drgplayercharacter))
              (`self.Release Actor Multicast`)
              (switch `/Game/ClawPerk/E_GrabbedObjectType` _type
                (:`NewEnumerator0`
                  (`self.K2_SetActorRotation` _target (`KismetMathLibrary.MakeRotator` 0.0 0.0 (.yaw (`PlayerCharacter.GetAimRotation` _drgplayercharacter))) false))
                (:`NewEnumerator1`
                  (`DeepPathfinderMovement.SetControlledExternally` (`DeepPathfinderCharacter.PathfinderMovement` _pathfindercharacter) false)))))
          (:`then_1`
            (`self.K2_DestroyActor` (`self.Handle`))))))))

(fn `Target Location`
  (returns (`Target Location` :type "Vector Structure"))
  (bind ((`Target_5_63C167034DFEE7C34BA8FFB2C364DDC8` _target)) (break `/Game/ClawPerk/F_MakeHookArgs` (`self.Make Hook Args`)))
  (switch `/Game/ClawPerk/E_ClawState` (`self.Claw State`)
    (:`NewEnumerator0`
      (`/Engine/EditorBlueprintResources/StandardMacros.IsValid` _target :!label _label
        (:`Is Valid`
          _)
        (:`Is Not Valid`
          (return (`self.Get Drop Point`)))))
    (:`NewEnumerator1`
      (goto _label))
    (:`NewEnumerator2`
      (return (`self.Get Drop Point`)))
    (:`NewEnumerator3`
      (return (`self.Get Drop Point`))))
  (return (+ (`self.K2_GetActorLocation` _target) (`self.Target Relative To Actor`))))

(fn `Update Grabbed Target`
  (bind ((`Target_5_63C167034DFEE7C34BA8FFB2C364DDC8` _target)) (break `/Game/ClawPerk/F_MakeHookArgs` (`self.Make Hook Args`)))
  (if (`self.Is Actor Grabbed`)
    (`/Engine/EditorBlueprintResources/StandardMacros.IsValid` _target
      (:`Is Valid`
        (`self.K2_SetActorLocation` _target (- (`self.K2_GetActorLocation`) (`self.Target Relative To Actor`)) false false))
      (:`Is Not Valid`
        (set `self.Is Actor Grabbed` false)))))

(fn `Update Rotation`
  (`SceneComponent.K2_SetWorldRotation` (`self.Grabber`) (`KismetMathLibrary.Conv_VectorToRotator` (`KismetMathLibrary.GetDirectionUnitVector` (`self.Get Drop Point`) (`self.Target Location`))) false false))

(fn `UserConstructionScript`)