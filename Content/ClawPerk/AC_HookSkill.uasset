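; Actor component for a Deep Rock Galactic claw perk that lets the player grab objects targeted with the Laser Pointer.
; While the pointer is equipped, it injects a GRAB label into the pointer's HUD, reflecting target grabbability and perk cooldown.
; The Cycleitem key plays the claw montage and spawns a hook on the aimed hit through the RPC spawner.
; The claw fires at the montage's "Fire" section and is destroyed on unequip.
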(event `self.ReceiveBeginPlay`)

(event `self.ReceiveTick`
  (params (DeltaSeconds :type "Float (single-precision)"))
  (bind _claw_actor (`self.Claw Actor`))
  (bind _drg_lib (`self.DRG Lib`))
  (`/Game/ClawPerk/ComponentMacros.Get DRG Lib Component` _drg_lib
    (:`Tick`
      (bind _aslaser_pointer_item (cast `LaserPointerItem` (`InventoryComponent.GetEquippedItem` (`PlayerCharacter.InventoryComponent` (`self.PlayerCharacter`))))
        (:`then`
          (`|ExecutionSequence`
            (:`then_0`
              (`/Engine/EditorBlueprintResources/StandardMacros.DoOnce` false
                (:`Completed`
                  (`self.Make Laser Pointer Label`))))
            (:`then_1`
              (`self.Update Laser Pointer Label` _aslaser_pointer_item))
            (:`then_2`
              (`self.Create Claw When Pressed` _aslaser_pointer_item))
            (:`then_3`
              (if (and (`KismetSystemLibrary.IsValid` (`self.Claw Actor`)) (== (`AnimInstance.Montage_GetCurrentSection` (`PlayerCharacter.GetFPAnimInstance` (`self.PlayerCharacter`)) "/Game/ClawPerk/Animations/Claw_Montage.Claw_Montage") "Fire"))
                (`/Engine/EditorBlueprintResources/StandardMacros.DoOnce` false :!label _label
                  (:`Completed`
                    (`/Game/ClawPerk/BP_Claw.Fire` (`self.Claw Actor`))))
                (else
                  (goto _label :!via `Reset`))))))
        (:`CastFailed`
          (`/Engine/EditorBlueprintResources/StandardMacros.IsValid` _claw_actor ; Destroy claw if the laser pointer is unequipped.
            (:`Is Valid`
              (`Actor.K2_DestroyActor` _claw_actor))))))
    (:`Init`
      (`/Game/DRGLib/LoggingFunctions/LIB_F_Log.AddLogEntry` _drg_lib "NewEnumerator2" "Hook" (`KismetStringLibrary.Concat_StrStr` "Value: " (`KismetStringLibrary.Conv_DoubleToString` (`self.FloatValue`))))
      (set `self.Hook Perk Asset` (`.Perk Asset` (`/Game/PerkLib/BP_PerkLibFunctionLibrary.Get Perk By Savegame ID` (`KismetGuidLibrary.Parse_StringToGuid` "06bc809f-732e-4c8f-a4ec-1766e1a685fc"))))
      (set `self.Player Controller` (`/Game/DRGLib/DRGFunctions/LIB_F_DRG.GetLocalPlayerController`))
      (bind (_found _spawner) (`/Game/ClawPerk/BP_ClawFunctionLibrary.Get Rpc Spawner`))
      (set `self.RPC Spawner` _spawner))))

(fn `Cool Down Time Left`
  (returns (`Time Left` :type "Float (double-precision)"))
  (return (`PerkAsset.GetUseCoolDownTimeLeft` (`self.Hook Perk Asset`) (`self.Player Controller`))))

(fn `Create Claw When Pressed`
  (params (`Laser Pointer` :type "LaserPointerItem Object Reference"))
  (if (and (== (`self.Cool Down Time Left`) 0.0) (`self.Hook Button Pressed`))
    (`self.Create Hook From Hit` (`LaserPointerItem.LookAtHit` `Laser Pointer`))))

(fn `Create Hook From Hit`
  (params (Hit :type "HitResult Structure"))
  (bind _claw_actor (`self.Claw Actor`))
  (bind (_bblockinghit _binitialoverlap _time _distance _location _impactpoint _normal _impactnormal _physmat _hitactor) (`GameplayStatics.BreakHitResult` (`local.Hit`)))
  (`|ExecutionSequence`
    (:`then_0`
      (`/Engine/EditorBlueprintResources/StandardMacros.IsValid` _claw_actor ; Destroy the claw if it was already created.
        (:`Is Valid`
          (`Actor.K2_DestroyActor` _claw_actor))))
    (:`then_1`
      (`AnimInstance.Montage_Play` (`PlayerCharacter.GetFPAnimInstance` (`self.PlayerCharacter`)) "/Game/ClawPerk/Animations/Claw_Montage.Claw_Montage" 1.0 "MontageLength" 0.0 false)
      (`/Game/ClawPerk/BP_RpcSpawner.Spawn Hook` (`self.RPC Spawner`) (`KismetMathLibrary.MakeTransform` (0.0 0.0 0.0)) (make `/Game/ClawPerk/F_MakeHookArgs` _hitactor _location (`self.Grabbed Object Info`) (make `/Game/ClawPerk/F_DrgContext` true (`self.Hook Perk Asset`) (`self.PlayerCharacter`)))))))

(fn `Hook Button Pressed`
  (returns (Pressed :type Boolean))
  (for _array_element (`InputSettings.GetActionMappingByName` (`InputSettings.GetInputSettings`) "Cycleitem")
    (if (`PlayerController.WasInputKeyJustPressed` (`self.Player Controller`) (`.Key` (break `InputActionKeyMapping` _array_element)))
      (return true)))
  (return false))

(fn `Make Laser Pointer Label`
  ;[0.2773 0.771 1] Add grab label to laser pointer screen
  (bind _aswpn_laser_pointer (cast `/Game/WeaponsNTools/LaserPointer/WPN_LaserPointer` (`InventoryComponent.LaserPointerItem` (`PlayerCharacter.InventoryComponent` (`self.PlayerCharacter`)))))
  (bind _returnvalue (`|CreateWidget` "/Game/UI/Global_UI_Elements/UI_AdvancedLabel.UI_AdvancedLabel_C")) ; Create the label
  (bind _output_get (set `self.Grab Label` _returnvalue))
  (`Widget.SetVisibility` _output_get "Hidden") ; Hide the label
  (`FSDAdvancedLabel.SetText` _output_get "[Cycleitem] GRAB" "") ; Label text
  (`/Game/UI/Global_UI_Elements/UI_AdvancedLabel.SetFont` _output_get (make `SlateFontInfo` "/Game/Art/Fonts/Acumin_Pro_Condensed.Acumin_Pro_Condensed" null (make `FontOutlineSettings` :`OutlineSize` 4) "Condensed Bold" 35) false) ; Set font
  (`/Game/UI/Global_UI_Elements/UI_AdvancedLabel.SetIconSize` _output_get 40 0)
  (bind _ascanvas_panel (cast `CanvasPanel` (`Widget.GetParent` (`Widget.GetParent` (`Widget.GetParent` (`Widget.GetParent` (`/Game/WeaponsNTools/LaserPointer/HUD_LaserPointerDisplay.LBL_LeftMouse` (`/Game/WeaponsNTools/LaserPointer/WPN_LaserPointer.HUD` _aswpn_laser_pointer)))))))) ; Get the laser pointer hud's canvas
  (`PanelWidget.AddChild` _ascanvas_panel _returnvalue) ; Add the grab label to the canvas
  (bind _ascanvas_panel_slot (cast `CanvasPanelSlot` (`Widget.Slot` _returnvalue))) ; Align grab label
  (`CanvasPanelSlot.SetAnchors` _ascanvas_panel_slot (make `Anchors` (0.5 0.0) (0.5 0.0)))
  (`CanvasPanelSlot.SetPosition` _ascanvas_panel_slot (0.0 63.0))
  (`CanvasPanelSlot.SetAlignment` _ascanvas_panel_slot (0.5 0.0)))

(fn `Update Laser Pointer Label`
  (params (self2 :type "LaserPointerItem Object Reference"))
  (bind _time_left (`self.Cool Down Time Left`))
  (bind _grab_label (`self.Grab Label`))
  (bind _output_get (set `self.Grabbed Object Info` (`/Game/ClawPerk/BP_ClawFunctionLibrary.Get Grabbed Actor Info` (`.HitActor` (`GameplayStatics.BreakHitResult` (`LaserPointerItem.LookAtHit` self2))))))
  (switch `/Game/ClawPerk/E_GrabbedObjectType` (`.Type_14_7B5B80B343C99BDA4E6C0DBD5E3A0210` (break `/Game/ClawPerk/F_GrabbedObjectInfo` _output_get))
    (:`NewEnumerator0`
      (`Widget.SetVisibility` _grab_label "Visible" :!label _label)
      (if (== _time_left 0.0)
        (`/Game/UI/Global_UI_Elements/UI_AdvancedLabel.SetTextTint` _grab_label (struct :`R` 0.210405 :`G` 0.9875 :`B` 0.19118 :`A` 1.0))
        (`FSDAdvancedLabel.SetText` _grab_label "[Cycleitem] GRAB" "") ; Label text
        (else
          (`/Game/UI/Global_UI_Elements/UI_AdvancedLabel.SetTextTint` _grab_label (struct :`R` 1.0 :`G` 0.135055 :`B` 0.158932 :`A` 0.7))
          (`FSDAdvancedLabel.SetText` _grab_label (`|FormatText` "[Cycleitem] GRAB ({0})" (`KismetMathLibrary.FCeil` _time_left)) "") ; Label text
        )))
    (:`NewEnumerator1`
      (goto _label))
    (:`NewEnumerator2`
      (goto _label))
    (:`NewEnumerator3`
      (goto _label))
    (:`NewEnumerator5`
      (goto _label))
    (:`NewEnumerator4`
      (`Widget.SetVisibility` _grab_label "Hidden"))))