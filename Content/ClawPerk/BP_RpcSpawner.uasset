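; BP_RpcSpawner spawns BP_Claw actors for the claw perk, keeping the spawn on the network authority.
; SpawnHook spawns directly with authority, while remote callers route through the SpawnHookServer event to the same DoSpawn function.
; DoSpawn creates the claw at the given transform and passes it through SpawnNotificationOwner to OnClawSpawned's NewClawConstructed.
; The hook arguments reach DoSpawn but are not applied to the spawned claw.
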(event `Spawn Hook`
  (params (SpawnTransform :type "Transform Structure") (`Make Hook Args` :type "/Game/ClawPerk/F_MakeHookArgs Structure"))
  (`/Engine/EditorBlueprintResources/ActorMacros.Switch Has Authority`
    (:`Authority`
      (`self.Do spawn` SpawnTransform `Make Hook Args`))
    (:`Remote`
      (`self.Spawn Hook Server` SpawnTransform `Make Hook Args`))))

(event `self.ReceiveBeginPlay`)

(event `Spawn Hook Server`
  (params (SpawnTransform :type "Transform Structure") (`Spawn Hook Args` :type "/Game/ClawPerk/F_MakeHookArgs Structure"))
  (`self.Do spawn` SpawnTransform `Spawn Hook Args`))

(event `Spawn Notification Owner`
  (params (Claw :type "/Game/ClawPerk/BP_Claw Object Reference"))
  (`/Game/ClawPerk/BI_ClawCreated.New Claw Constructed` (`self.On Claw Spawned`) Claw))

(fn `Do spawn`
  (params (SpawnTransform :type "Transform Structure") (`Spawn Hook Args` :type "/Game/ClawPerk/F_MakeHookArgs Structure"))
  (bind _returnvalue (`|SpawnActorFromClass` "/Game/ClawPerk/BP_Claw.BP_Claw_C" SpawnTransform "Undefined" "OverrideRootScale" null null))
  (`self.Spawn Notification Owner` _returnvalue))

(fn `UserConstructionScript`)