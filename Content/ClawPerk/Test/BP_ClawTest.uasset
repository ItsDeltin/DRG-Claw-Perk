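; BP_ClawTest is a test actor for spawning and firing the claw perk's hook at a TestTarget.
; MakeHook asks the RPC spawner to spawn a hook, passing itself as adapter, after a zero-second delay that works around server calls from editor buttons.
; Setup stores the resulting claw and builds it from hardcoded pickaxe part meshes.
; FireHook fires that claw, and GetDropRotation supplies the actor's rotation.
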(event `Make Hook`
  (bind _test_target (`self.Test Target`))
  (`KismetSystemLibrary.Delay` 0.0) ; hacky workaround :D\nsomething goes wack when calling server\nusing editor buttons, this fixes it :D :D :D :D \nspent 6 hours on this i did
  (bind (_found _spawner) (`/Game/ClawPerk/BP_ClawFunctionLibrary.Get Rpc Spawner`))
  (if _found
    (`/Game/ClawPerk/BP_RpcSpawner.Spawn Hook` _spawner (`self.GetTransform`) (make `/Game/ClawPerk/F_MakeHookArgs` self _test_target (`self.K2_GetActorLocation` _test_target)))))

(event `self.ReceiveBeginPlay`)

(event `self.ReceiveTick`
  (params (DeltaSeconds :type "Float (single-precision)")))

(event `/Game/ClawPerk/Adapter/BI_ClawAdapter.Setup`
  (params (BP_Claw :type "/Game/ClawPerk/BP_Claw Object Reference"))
  (bind _output_get (set `self.BP_Claw` BP_Claw))
  (`/Game/ClawPerk/BP_Claw.Make Hook` _output_get (`|MakeMap` "Head" "/Game/ClawPerk/TestAssets/drg_hook_SM_Pickaxe_Head_ArcWelders_S01_mo.drg_hook_SM_Pickaxe_Head_ArcWelders_S01_mo" "Shaft" "/Game/ClawPerk/TestAssets/drg_hook_SM_PickAxe_Shaft_009_mo.drg_hook_SM_PickAxe_Shaft_009_mo" "FrontBlade" "/Game/ClawPerk/TestAssets/drg_hook_SM_PickAxe_BladeFront_005_mo.drg_hook_SM_PickAxe_BladeFront_005_mo" "BackBlade" "/Game/ClawPerk/TestAssets/drg_hook_SM_PickAxe_BladeSpecial_Chasmborne_mo.drg_hook_SM_PickAxe_BladeSpecial_Chasmborne_mo" "Handle" "/Game/ClawPerk/TestAssets/drg_hook_SM_PickAxe_Handle_ReapersClaw_mo.drg_hook_SM_PickAxe_Handle_ReapersClaw_mo" "Pommel" "/Game/ClawPerk/TestAssets/drg_hook_SM_PickAxe_Pommel_ReapersClaw_mo.drg_hook_SM_PickAxe_Pommel_ReapersClaw_mo" :!type "EPickaxePartLocation Enum" :!valuetype "StaticMesh Object Reference") null)
  (`KismetSystemLibrary.PrintString` "Local ClawTest got new hook"))

(fn `Fire Hook`
  (`/Engine/EditorBlueprintResources/StandardMacros.IsValid` (`self.BP_Claw`)
    (:`Is Valid`
      (`/Game/ClawPerk/BP_Claw.Fire` (`self.BP_Claw`)))
    (:`Is Not Valid`
      (`KismetSystemLibrary.PrintString` "Can't fire claw; claw not created."))))

(fn `Get Drop Rotation`
  (returns (Rotation :type "Rotator Structure"))
  (bind (_returnvalue_location _returnvalue_rotation) (`KismetMathLibrary.BreakTransform` (`self.GetTransform`)))
  (return _returnvalue_rotation))

(fn `UserConstructionScript`)