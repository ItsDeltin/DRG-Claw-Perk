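; Claw perk hook actor for a Deep Rock Galactic mod, built from pickaxe-part pieces, that grabs targets and reels them to the player.
; Server-initiated multicast fires it; Tick drives Extending, Retracting and Completed movement, detaching from and reattaching to the claw item.
; Grabbed actors follow the hook, except physics carriables and players, which get velocity while the hook follows them.
; Release spends a perk charge and uses or picks up items.
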(event `self.ReceiveBeginPlay`
  (bind _pickaxe_part_location_to_static_mesh (`/Game/ClawPerk/BP_ClawFunctionLibrary.Get Editor Pickaxe Part Testing Array`))
  (bind _claw_pieces (`self.Get Model Pieces`))
  (bind _grabber (`self.Grabber`))
  (bind _player_character (`self.Player Character`))
  ;[1 0.04062 0.04062] Begin Play
  (bind _created_components (`/Game/ClawPerk/BP_ClawFunctionLibrary.Make Pieces from Player Character` _player_character _grabber _claw_pieces _pickaxe_part_location_to_static_mesh true)) ; First person
  (set `self.Hook Pieces` _created_components)
  (`/Game/ClawPerk/BP_ClawFunctionLibrary.Make Pieces from Player Character` _player_character _grabber _claw_pieces _pickaxe_part_location_to_static_mesh) ; Third person
  (set `self.Perk Asset` (`.Perk Asset` (`/Game/PerkLib/BP_PerkLibFunctionLibrary.Get Perk By Savegame ID` (`KismetGuidLibrary.Parse_StringToGuid` "06bc809f-732e-4c8f-a4ec-1766e1a685fc"))))
  (`/Game/ClawPerk/BP_ClawFunctionLibrary.Dev Log` "Hook spawned"))

(event `self.ReceiveTick`
  (params (DeltaSeconds :type "Float (single-precision)"))
  (bind _target_location (`self.Target Location`))
  (bind _returnvalue (`self.K2_GetActorLocation`))
  (bind _target_actor (`self.Target Actor`))
  (bind _itm_claw (`self.Itm Claw`))
  (bind ((`Type_14_7B5B80B343C99BDA4E6C0DBD5E3A0210` _type) (`PlayerCharacter_20_8E807B09428E3040D6646386625F92E0` _playercharacter)) (break `/Game/ClawPerk/F_GrabbedObjectInfo` (`self.Grabbed Object Info`)))
  (bind _returnvalue_2 (`self.K2_GetActorLocation` (`self.Target Actor`)))
  (bind _returnvalue_3 (`KismetMathLibrary.Vector_Distance` _returnvalue _target_location))
  (bind _returnvalue_4 (* (`KismetMathLibrary.GetDirectionUnitVector` _returnvalue_2 _target_location) (`self.Distance Per Second`)))
  ;[1 0 0.008587] Event Tick
  (`|ExecutionSequence`
    (:`then_0`
      (`/Engine/EditorBlueprintResources/StandardMacros.IsValid` _itm_claw
        (:`Is Valid`
          (switch `/Game/ClawPerk/E_ClawState` (`self.Claw State`)
            (:`NewEnumerator0`
              _)
            (:`NewEnumerator1`
              _)
            (:`NewEnumerator2`
              _)
            (:`NewEnumerator3`
              (`/Engine/EditorBlueprintResources/StandardMacros.DoOnce` false :!label _label
                (:`Completed`
                  (`self.K2_AttachToComponent` (`/Game/ClawPerk/Item/ITM_Claw.Attach Point` _itm_claw) "None" "SnapToTarget" "KeepWorld" "KeepRelative")
                  (goto _label_2 :!via `Reset`)))))
          (`|ExecutionSequence`
            (:`then_0`
              (`/Engine/EditorBlueprintResources/StandardMacros.DoOnce` false :!label _label_2 ; This is executed once the hook is fired.\nIt's kind of weird to put this here instead of wherever the state changes.
                (:`Completed`
                  (`self.K2_DetachFromActor` "KeepWorld" "KeepWorld"))))
            (:`then_1`
              (goto _label :!via `Reset`))
            (:`then_2`
              (if (`self.Should Physically Retract`)
                (`self.K2_SetActorLocation` (- _returnvalue_2 (`self.Target Relative To Actor`)))
                (else
                  (`self.K2_SetActorLocation` (+ _returnvalue (* (`KismetMathLibrary.GetDirectionUnitVector` _returnvalue _target_location) (`KismetMathLibrary.FMin` _returnvalue_3 (* (`self.Distance Per Second`) DeltaSeconds)))))))
              (`|ExecutionSequence`
                (:`then_0`
                  (if (`self.Is Actor Grabbed`)
                    (`/Engine/EditorBlueprintResources/StandardMacros.IsValid` _target_actor ; Make sure the target is still valid.
                      (:`Is Valid`
                        (switch `/Game/ClawPerk/E_GrabbedObjectType` _type
                          (:`NewEnumerator0`
                            (`self.K2_SetActorLocation` _target_actor (- (`self.K2_GetActorLocation`) (`self.Target Relative To Actor`)) false false :!label _label_3))
                          (:`NewEnumerator1`
                            (goto _label_3))
                          (:`NewEnumerator2`
                            (goto _label_3))
                          (:`NewEnumerator3`
                            (bind _asprimitive_component (cast `PrimitiveComponent` (`Actor.RootComponent` _target_actor))
                              (:`then`
                                (`PrimitiveComponent.SetPhysicsLinearVelocity` _asprimitive_component _returnvalue_4 false "None"))
                              (:`CastFailed`
                                (goto _label_3))))
                          (:`NewEnumerator5`
                            (goto _label_3))
                          (:`NewEnumerator6`
                            (`PrimitiveComponent.SetPhysicsLinearVelocity` (`Character.CapsuleComponent` _playercharacter) _returnvalue_4 false "None"))))
                      (:`Is Not Valid`
                        (set `self.Is Actor Grabbed` false)))))
                (:`then_1`
                  (if (or (and (`self.Should Physically Retract`) (< _returnvalue_3 200.0)) (< _returnvalue_3 (`self.Distance Tolerance`)))
                    (switch `/Game/ClawPerk/E_ClawState` (`self.Claw State`)
                      (:`NewEnumerator0`
                        (`self.Grab Target`)
                        (`self.Retract Multicast`))
                      (:`NewEnumerator2`
                        (`self.Release Target`)
                        (set `self.Claw State` "NewEnumerator3")
                        (`self.Set Enabled FP Fov` true)
                        (`/Game/ClawPerk/Item/ITM_Claw.Hide Cable` (`self.Itm Claw`))))))))))))
    (:`then_1`
      (if (not (`self.IsActorBeingDestroyed`))
        (`|ExecutionSequence`
          (:`then_0`
            ;;[1 0.4641 0.1309] Client hook position > server position
            (if (not (== (`self.Claw State`) (enumliteral `/Game/ClawPerk/E_ClawState` "NewEnumerator3")))
              (bind (_direction _lerp_between_client_and_true_position) (`Timeline|luna tuna`)
                (:`Update`
                  (set `self.Attach Point to Real Point lerp` _lerp_between_client_and_true_position)))))
          (:`then_1`))))))

(event `Fire Multicast`
  (params (`Grabbed Object Info` :type "/Game/ClawPerk/F_GrabbedObjectInfo Structure") (`Target Actor` :type "Actor Object Reference") (`Target Relative To Actor` :type "Vector Structure"))
  ;[1 0.1432 0.7478] Fire (Multicast)
  (set `self.Grabbed Object Info` `Grabbed Object Info`)
  (set `self.Target Actor` `Target Actor`)
  (set `self.Target Relative To Actor` `Target Relative To Actor`)
  (set `self.Claw State` "NewEnumerator0")
  (`self.Update Rotation`)
  (`self.Set Enabled FP Fov` false)
  (`/Game/ClawPerk/BP_ClawFunctionLibrary.Dev Log` (`KismetStringLibrary.Concat_StrStr` "[mutlicast] hook fired! \nTarget: " (`KismetSystemLibrary.GetDisplayName` `Target Actor`) " \nTarget relative to actor: " (`KismetStringLibrary.Conv_VectorToString` `Target Relative To Actor`) " \nType: " (`|GetEnumeratorNameAsString` (`.Type_14_7B5B80B343C99BDA4E6C0DBD5E3A0210` (break `/Game/ClawPerk/F_GrabbedObjectInfo` `Grabbed Object Info`))))))

(event `Fire Server`
  (params (`Grabbed Object Info` :type "/Game/ClawPerk/F_GrabbedObjectInfo Structure") (`Target Actor` :type "Actor Object Reference") (`Target Location` :type "Vector Structure"))
  ;[1 0.3862 0.003982] Fire (Server)
  (`self.Fire Multicast` `Grabbed Object Info` `Target Actor` (- `Target Location` (`self.K2_GetActorLocation` `Target Actor`)))
  (`/Game/ClawPerk/BP_ClawFunctionLibrary.Dev Log` "[server] hook fired!"))

(event `Grab Multicast`
  (params (`Was Grabbed` :type Boolean))
  ;[1 0.1949 0.8564] On Grab (Multicast)
  (set `self.Is Actor Grabbed` `Was Grabbed`))

(event `Retract Multicast`
  ;[1 0.2581 0.7427] Retract (Multicast)
  (set `self.Claw State` "NewEnumerator2"))

(event `Release Actor Multicast`
  (bind _player_character (`self.Player Character`))
  (bind ((`Type_14_7B5B80B343C99BDA4E6C0DBD5E3A0210` _type) (`CollectibleBase_11_74E9D1714E7BF2CDEC71368D4724A985` _collectiblebase) (`CarriableComponent_6_1B3B74D546E577A40FD1DDBC77F5E328` _carriablecomponent) (`UsableComponent_17_0CAA5EFE47645D7BC28A96A332A2E1E6` _usablecomponent)) (break `/Game/ClawPerk/F_GrabbedObjectInfo` (`self.Grabbed Object Info`)))
  ;[1 0.3515 0.9126] Release Actor (Multicast)
  (switch `/Game/ClawPerk/E_GrabbedObjectType` _type
    (:`NewEnumerator2`
      (`UsableComponentBase.BeginUse` (`/Game/GameElements/Resources/Collectibles/BP_Collectible_Base.InstantUsable` _collectiblebase) _player_character "Use"))
    (:`NewEnumerator3`
      (`CarriableComponent.PickupItem` _carriablecomponent _player_character))
    (:`NewEnumerator5`
      (`SingleUsableComponent.Use` _usablecomponent _player_character "Use" 1.0)
      (`UsableComponentBase.BeginUse` (`self.Fake Usable`) _player_character "Use"))))

(fn `Fire`
  (params (`Grabbed Object Info` :type "/Game/ClawPerk/F_GrabbedObjectInfo Structure") (`Target Actor` :type "Actor Object Reference") (`Target Location` :type "Vector Structure"))
  (`/Engine/EditorBlueprintResources/ActorMacros.Switch Has Authority`
    (:`Authority`
      (`self.Fire Server` `Grabbed Object Info` `Target Actor` `Target Location`))))

(fn `Get Drop Point`
  (returns (`Drop Location` :type "Vector Structure"))
  (bind _itm_claw (`self.Itm Claw`))
  (bind _player_character (`self.Player Character`))
  (`/Engine/EditorBlueprintResources/StandardMacros.IsValid` _player_character
    (:`Is Valid`
      (return (+ (* (`KismetMathLibrary.GetForwardVector` (`PlayerCharacter.GetAimRotation` _player_character)) 100.0) (`SceneComponent.K2_GetComponentLocation` (`PlayerCharacter.FirstPersonRoot` _player_character)))))
    (:`Is Not Valid`
      (return (+ (`self.K2_GetActorLocation` _itm_claw) (* (`KismetMathLibrary.GetForwardVector` (`self.K2_GetActorRotation` _itm_claw)) 100.0))))))

(fn `Get Model Pieces`
  (returns (`Claw Pieces` :type "Array of /Game/ClawPerk/F_ClawPiece Structure"))
  (bind _shaft_relative_transform (`self.Shaft Relative Transform`))
  (bind _blade_relative_transform (`self.Blade Relative Transform`))
  (return (`|MakeArray` (make `/Game/ClawPerk/F_ClawPiece` "Head" "Bone-Base" (`self.Head Relative Transform`)) (make `/Game/ClawPerk/F_ClawPiece` "Shaft" "Bone-Front-Shaft" _shaft_relative_transform) (make `/Game/ClawPerk/F_ClawPiece` "Shaft" "Bone-Special-Shaft" (`KismetMathLibrary.ComposeTransforms` _shaft_relative_transform (`KismetMathLibrary.MakeTransform` (0.0 0.0 0.0)))) (make `/Game/ClawPerk/F_ClawPiece` "FrontBlade" "Bone-Front" _blade_relative_transform) (make `/Game/ClawPerk/F_ClawPiece` "BackBlade" "Bone-Special" (`KismetMathLibrary.ComposeTransforms` _blade_relative_transform (`KismetMathLibrary.MakeTransform` (0.0 0.0 0.0) (struct :`Pitch` 180.0)))))))

(fn `Grab Target`
  (bind ((`Type_14_7B5B80B343C99BDA4E6C0DBD5E3A0210` _type) (`PathfinderCharacter_2_25853F2D40E1B0E7C83EB18A9FC05298` _pathfindercharacter)) (break `/Game/ClawPerk/F_GrabbedObjectInfo` (`self.Grabbed Object Info`)))
  (bind _output_get (set `self.Is Actor Grabbed` (`|EnumInequality` _type (enumliteral `/Game/ClawPerk/E_GrabbedObjectType` "NewEnumerator4"))))
  (`self.Grab Multicast` _output_get)
  (if _output_get
    (switch `/Game/ClawPerk/E_GrabbedObjectType` _type
      (:`NewEnumerator1`
        (`DeepPathfinderMovement.SetControlledExternally` (`DeepPathfinderCharacter.PathfinderMovement` _pathfindercharacter) true) ; Allows us to move pathfinder characters
      ))))

(fn `Release Target`
  (bind _player_character (`self.Player Character`))
  (bind ((`Type_14_7B5B80B343C99BDA4E6C0DBD5E3A0210` _type) (`PathfinderCharacter_2_25853F2D40E1B0E7C83EB18A9FC05298` _pathfindercharacter)) (break `/Game/ClawPerk/F_GrabbedObjectInfo` (`self.Grabbed Object Info`)))
  (if (`self.Is Actor Grabbed`)
    (set `self.Is Actor Grabbed` false)
    (`/Engine/EditorBlueprintResources/ActorMacros.Switch Has Authority`
      (:`Authority`
        (if true
          (`PerkAsset.UseCharge` (`self.Perk Asset`) (`PlayerCharacter.GetPlayerController` _player_character))
          (`self.Release Actor Multicast`)
          (switch `/Game/ClawPerk/E_GrabbedObjectType` _type
            (:`NewEnumerator0`
              (`self.K2_SetActorRotation` (`self.Target Actor`) (`KismetMathLibrary.MakeRotator` 0.0 0.0 (.yaw (`PlayerCharacter.GetAimRotation` _player_character))) false))
            (:`NewEnumerator1`
              (`DeepPathfinderMovement.SetControlledExternally` (`DeepPathfinderCharacter.PathfinderMovement` _pathfindercharacter) false))))))))

(fn `Set Enabled FP Fov`
  (params (`Enabled FPFOV` :type Boolean))
  (for _array_element (`self.Hook Pieces`)
    (set `FirstPersonStaticMeshComponent.EnabledFPFOV` `Enabled FPFOV` _array_element)))

(fn `Set State`
  (params (`New State` :type "/Game/ClawPerk/E_ClawState Enum" :default "NewEnumerator0"))
  (bind _output_get (set `self.Claw State` `New State`))
  (switch `/Game/ClawPerk/E_ClawState` _output_get
    (:`NewEnumerator0`
      (`self.Set Enabled FP Fov` false :!label _label))
    (:`NewEnumerator1`
      (goto _label))
    (:`NewEnumerator2`
      (goto _label))
    (:`NewEnumerator3`
      (`self.Set Enabled FP Fov` true))))

(fn `Should Physically Retract`
  (returns (`Do Physically Retract` :type Boolean))
  (bind ((`Type_14_7B5B80B343C99BDA4E6C0DBD5E3A0210` _type)) (break `/Game/ClawPerk/F_GrabbedObjectInfo` (`self.Grabbed Object Info`)))
  (return (and (or (== (enumliteral `/Game/ClawPerk/E_GrabbedObjectType` "NewEnumerator3") _type) (`|EnumEquality` (enumliteral `/Game/ClawPerk/E_GrabbedObjectType` "NewEnumerator6") _type)) (`self.Is Actor Grabbed`) (`|EnumEquality` (`self.Claw State`) "NewEnumerator2"))))

(fn `Target Location`
  (returns (`Target Location` :type "Vector Structure"))
  (bind _target_actor (`self.Target Actor`))
  (switch `/Game/ClawPerk/E_ClawState` (`self.Claw State`)
    (:`NewEnumerator0`
      (`/Engine/EditorBlueprintResources/StandardMacros.IsValid` _target_actor :!label _label
        (:`Is Valid`
          _)
        (:`Is Not Valid`
          (return (`self.Get Drop Point`)))))
    (:`NewEnumerator1`
      (goto _label))
    (:`NewEnumerator2`
      (return (`self.Get Drop Point`)))
    (:`NewEnumerator3`
      (return (`self.Get Drop Point`))))
  (return (+ (`self.K2_GetActorLocation` _target_actor) (`self.Target Relative To Actor`))))

(fn `Update Grabbed Target`
  (bind _target_actor (`self.Target Actor`))
  (bind ((`Type_14_7B5B80B343C99BDA4E6C0DBD5E3A0210` _type) (`PlayerCharacter_20_8E807B09428E3040D6646386625F92E0` _playercharacter)) (break `/Game/ClawPerk/F_GrabbedObjectInfo` (`self.Grabbed Object Info`)))
  (if (`self.Is Actor Grabbed`)
    (`/Engine/EditorBlueprintResources/StandardMacros.IsValid` _target_actor
      (:`Is Valid`
        (switch `/Game/ClawPerk/E_GrabbedObjectType` _type
          (:`NewEnumerator0`
            (`self.K2_SetActorLocation` _target_actor (- (`self.K2_GetActorLocation`) (`self.Target Relative To Actor`)) false false :!label _label))
          (:`NewEnumerator1`
            (goto _label))
          (:`NewEnumerator2`
            (goto _label))
          (:`NewEnumerator3`
            (goto _label))
          (:`NewEnumerator5`
            (goto _label))
          (:`NewEnumerator6`
            (`PrimitiveComponent.SetPhysicsLinearVelocity` (`Character.CapsuleComponent` _playercharacter) (0.0 0.0 0.0) false "None"))))
      (:`Is Not Valid`
        (set `self.Is Actor Grabbed` false)))))

(fn `Update Rotation`
  (`SceneComponent.K2_SetWorldRotation` (`self.Grabber`) (`KismetMathLibrary.Conv_VectorToRotator` (`KismetMathLibrary.Cross_VectorVector` (`KismetMathLibrary.GetDirectionUnitVector` (`self.Get Drop Point`) (`self.Target Location`)) (`KismetMathLibrary.Vector_Up`))) false false))

(fn `UserConstructionScript`)