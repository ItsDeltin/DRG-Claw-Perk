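; Function library for creating and looking up perks at runtime, built on the game's FSD data.
; CreateFloatPerk constructs a FloatPerkAsset outered to the game data, fills it from the supplied parameters, then passes it to the InitSpacerig actor's AddFloatPerk.
; GetPerkBySavegameID searches the game data's perk assets for a matching savegame ID and returns whether it exists along with the asset.
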(fn `Create Float Perk`
  (params (SaveGameID :type "Guid Structure") (Title :type Text) (Icon :type "Texture2D Object Reference") (bIsEquippable :type Boolean) (ShoutOnUseCharge :type "DialogDataAsset Object Reference") (PerkLogicClasses :type "Array of PerkLogic Soft Class Reference") (HudIconWidgetClass :type "PerkHUDIconWidget Soft Class Reference") (`Hud Activation Widgets` :type "Array of PerkHUDActivationWidget Soft Class Reference") (MaxUseCharges :type Integer) (CoolDownBetweenUse :type "Float (double-precision)") (bIsHighlighted :type Boolean) (Effects :type "Array of FloatPerkEffect Structure") (Ranks :type "Array of FloatPerkRank Structure"))
  (bind _returnvalue (`|GenericCreateObject` "/Script/FSD.FloatPerkAsset" (`GameFunctionLibrary.GetFSDGameData`)))
  (set `PerkAsset.SavegameID` SaveGameID _returnvalue)
  (set `PerkAsset.Title` Title _returnvalue)
  (set `PerkAsset.Icon` Icon _returnvalue)
  (set `PerkAsset.bIsEquippable` bIsEquippable _returnvalue)
  (set `PerkAsset.ShoutOnUseCharge` ShoutOnUseCharge _returnvalue)
  (set `PerkAsset.PerkLogicClasses` PerkLogicClasses _returnvalue)
  (set `PerkAsset.HudIconWidgetClass` HudIconWidgetClass _returnvalue)
  (set `PerkAsset.HudActivationWidgets` `Hud Activation Widgets` _returnvalue)
  (set `PerkAsset.MaxUseCharges` MaxUseCharges _returnvalue)
  (set `PerkAsset.CoolDownBetweenUse` CoolDownBetweenUse _returnvalue)
  (set `PerkAsset.bIsHighlighted` bIsHighlighted _returnvalue)
  (set `FloatPerkAsset.Effects` Effects _returnvalue)
  (set `FloatPerkAsset.Ranks` Ranks _returnvalue)
  (bind _returnvalue_2 (`GameplayStatics.GetActorOfClass` null "/Game/PerkLib/InitSpacerig.InitSpacerig_C"))
  (`/Game/PerkLib/InitSpacerig.Add Float Perk` _returnvalue_2 _returnvalue))

(fn `Get Perk By Savegame ID`
  (params (`Savegame ID` :type "Guid Structure"))
  (returns (Exists :type Boolean) (`Perk Asset` :type "PerkAsset Object Reference"))
  (for _array_element (`.PerkAssets` (break `GDPerks` (`GameData.perks` (`GameFunctionLibrary.GetFSDGameData`))))
    (if (== (`PerkAsset.SavegameID` _array_element) `Savegame ID`)
      (return true _array_element)))
  (return false null))